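; BP_Test17_Command is a test blueprint that drives the player's inventory through a command-style interface.
; On BeginPlay it casts the player pawn to BP_Test16_Character2 and caches its inventory component.
; Its Add, Move, Drop and Money events each call the component's single ExecuteCommand with a command type and matching parameters, with Drop using the pawn's location as the drop position.
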(event Custom|CommandAdd
  (Class|InventoryComponent|ExecuteCommand (Variables|Default|GetInventoryComp) (Utilities|Struct|MakeInventoryCommand "Add" (Variables|CommandTest|Add|GetCount) (Variables|CommandTest|Add|GetItemData) 1 1 "0.000000,0.000000,0.000000")))

(event Custom|CommandMove
  (Class|InventoryComponent|ExecuteCommand (Variables|Default|GetInventoryComp) (Utilities|Struct|MakeInventoryCommand "Move" 1 0 (Variables|CommandTest|Move|GetSourceIndex) (Variables|CommandTest|Move|GetTargetIndex) "0.000000,0.000000,0.000000")))

(event Custom|CommandDrop
  (Class|InventoryComponent|ExecuteCommand (Variables|Default|GetInventoryComp) (Utilities|Struct|MakeInventoryCommand "Drop" 1 0 (Variables|CommandTest|Drop|GetDropIndex) 1 (Transformation|GetActorLocation (Game|Player|GetPlayerPawn 0)))))

(event Custom|CommandMoney
  (Class|InventoryComponent|ExecuteCommand (Variables|Default|GetInventoryComp) (Utilities|Struct|MakeInventoryCommand "Money" (Variables|CommandTest|Money|GetMoneyDiff) 0 1 1 "0.000000,0.000000,0.000000")))

(event EventBeginPlay
  (bind _asbp_test_16_character_2 (Utilities|Casting|CastToBP_Test16_Character2 (Game|Player|GetPlayerPawn 0)))
  (Variables|Default|SetInventoryComp (Class|ActionCharacter|GetInventoryComponent _asbp_test_16_character_2)))

(fn ConstructionScript)