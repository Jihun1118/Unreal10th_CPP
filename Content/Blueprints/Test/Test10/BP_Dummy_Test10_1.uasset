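; BP_Dummy_Test10_1 is a test dummy actor that reports the damage it receives.
; Its AnyDamage event prints the damage amount, instigator and damage causer, then passes the amount to PlayPopup on the WBP_Test_DamagePopup held by its Widget component.
; A duplicate OnTakeAnyDamage handler only prints the same details, and its binding node is never executed.
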(event Custom|OnTakeAnyDamage_Event
  (params (DamagedActor :type Actor%20Object%20Reference) (Damage :type Float%20%28single-precision%29) (DamageType :type Damage%20Type%20Object%20Reference) (InstigatedBy :type Controller%20Object%20Reference) (DamageCauser :type Actor%20Object%20Reference))
  (Development|PrintString (Utilities|String|BuildString(Object) (Utilities|String|BuildString(Object) (Class|KismetStringLibrary|BuildStringDouble "" "Damage:" Damage ",") "Instigator : " InstigatedBy ",") "DamageCauser : " DamageCauser)))

(event EventBeginPlay)

(event Collision|EventActorBeginOverlap
  (params (OtherActor :type Actor%20Object%20Reference)))

(event EventTick
  (params (DeltaSeconds :type Float%20%28single-precision%29)))

(event Game|Damage|EventAnyDamage
  (params (Damage :type Float%20%28single-precision%29) (DamageType :type Damage%20Type%20Object%20Reference) (InstigatedBy :type Controller%20Object%20Reference) (DamageCauser :type Actor%20Object%20Reference))
  (Development|PrintString (Utilities|String|BuildString(Object) (Utilities|String|BuildString(Object) (Class|KismetStringLibrary|BuildStringDouble "" "Damage:" Damage ",") "Instigator : " InstigatedBy ",") "DamageCauser : " DamageCauser))
  (bind _aswbp_damage_popup (Utilities|Casting|CastToWBP_Test_DamagePopup (UserInterface|GetWidget (Variables|Default|GetWidget))))
  (Default|PlayPopup _aswbp_damage_popup Damage))

(fn ConstructionScript)