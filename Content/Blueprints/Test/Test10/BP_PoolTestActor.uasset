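; BP_PoolTestActor is a test actor for exercising spawn and return through the ObjectPoolSubsystem.
; OnSpawn makes it visible, enables collision and tick, then returns it to the pool after a short delay.
; OnReturn hides it and disables collision and tick, so it is deactivated rather than destroyed.
; Both events print debug messages to show when each pool transition fires.
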(event EventBeginPlay)

(event Collision|EventActorBeginOverlap
  (params (OtherActor :type Actor%20Object%20Reference)))

(event EventTick
  (params (DeltaSeconds :type Float%20%28single-precision%29)))

(event EventOnSpawn
  (Development|PrintString "OnSpawn : Test")
  (Rendering|SetActorHiddenInGame false)
  (Collision|SetActorEnableCollision true)
  (Actor|Tick|SetActorTickEnabled true)
  (Utilities|FlowControl|Delay 3.0)
  (Class|ObjectPoolSubsystem|ReturnPool (Subsystems|GetObjectPoolSubsystem) self))

(event EventOnReturn
  (Rendering|SetActorHiddenInGame true)
  (Collision|SetActorEnableCollision false)
  (Actor|Tick|SetActorTickEnabled false)
  (Development|PrintString "OnReturn : Test"))

(fn ConstructionScript)