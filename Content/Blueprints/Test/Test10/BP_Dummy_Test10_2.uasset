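; BP_Dummy_Test10_2 is a test dummy that reacts to damage by logging it and showing a damage popup.
; Its AnyDamage event prints the amount, instigator and causer, then spawns a PopupWidgetClass actor at the Scene component's transform, passing in the damage.
; A second handler prints the same string, but its OnTakeAnyDamage binding is disconnected and never runs.
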(event Custom|OnTakeAnyDamage_Event
  (params (DamagedActor :type Actor%20Object%20Reference) (Damage :type Float%20%28single-precision%29) (DamageType :type Damage%20Type%20Object%20Reference) (InstigatedBy :type Controller%20Object%20Reference) (DamageCauser :type Actor%20Object%20Reference))
  (Development|PrintString (Utilities|String|BuildString(Object) (Utilities|String|BuildString(Object) (Class|KismetStringLibrary|BuildStringDouble "" "Damage:" Damage ",") "Instigator : " InstigatedBy ",") "DamageCauser : " DamageCauser)))

(event EventBeginPlay)

(event Collision|EventActorBeginOverlap
  (params (OtherActor :type Actor%20Object%20Reference)))

(event EventTick
  (params (DeltaSeconds :type Float%20%28single-precision%29)))

(event Game|Damage|EventAnyDamage
  (params (Damage :type Float%20%28single-precision%29) (DamageType :type Damage%20Type%20Object%20Reference) (InstigatedBy :type Controller%20Object%20Reference) (DamageCauser :type Actor%20Object%20Reference))
  (Development|PrintString (Utilities|String|BuildString(Object) (Utilities|String|BuildString(Object) (Class|KismetStringLibrary|BuildStringDouble "" "Damage:" Damage ",") "Instigator : " InstigatedBy ",") "DamageCauser : " DamageCauser))
  (Game|SpawnActorfromClass (Variables|Default|GetPopupWidgetClass) (Transformation|GetWorldTransform (Variables|Default|GetScene)) "Undefined" "MultiplyWithRoot" 0 Damage 0))

(fn ConstructionScript)